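; Clickable hotspot in the car configurator that toggles an open/close animation on a part of the BP_AudiA5.
; PlayAnimation reads sounds, speeds and wait time from a DataTable, blocks opening while dependencies animate, and force-closes a linked focus point.
; Open and Close shift the actor by an offset and set a material hide timer.
; Tick times animations and presses, and drives marker visibility from mouse screen distance and optional camera facing.
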(event `self.ReceiveBeginPlay`
  (bind _plane (`self.Plane`))
  ;[1 1 1] Apply Dynamic material
  (bind _returnvalue (`PrimitiveComponent.CreateDynamicMaterialInstance` _plane 0 (`PrimitiveComponent.GetMaterial` _plane 0) "None"))
  (bind _output_get (set `self.DynamicMaterialInstance` _returnvalue))
  (`MaterialInstanceDynamic.SetScalarParameterValue` _output_get "Scale" (`self.Scale`)))

(event `PlayAnimation`
  (bind _closedependency (`self.CloseDependency`))
  ;[1 1 1] Play animation
  (`|ExecutionSequence`
    (:`then_0`
      (`self.GetCarInstance`)
      (if (and (`self.CanBeAnimated`) (not (`self.IsAnimating`)))
        (`self.GetAnimationData`)
        (if (`self.IsOpen`)
          (`self.Close`)
          (else
            ;[1 1 1] Check open dependencies before opening
            (set `self.CanBeOpened` true)
            (for _array_element (`self.OpenDependency`)
              (`/Engine/EditorBlueprintResources/StandardMacros.IsValid` _array_element
                (:`Is Valid`
                  (if (`/Game/CarConfigurator/Shared/Blueprints/BP_FocusPoint.IsAnimating` _array_element)
                    (set `self.CanBeOpened` false)))))
            (if (`self.CanBeOpened`)
              (`self.Open`))))))
    (:`then_1`
      ;[1 1 1] Force close these dependencies
      (`/Engine/EditorBlueprintResources/StandardMacros.IsValid` _closedependency
        (:`Is Valid`
          (if (`/Game/CarConfigurator/Shared/Blueprints/BP_FocusPoint.IsOpen` _closedependency)
            (`self.ForceClose` _closedependency)))))))

(event `self.ReceiveTick`
  (params (DeltaSeconds :type "Float (single-precision)"))
  (bind _dynamicmaterialinstance (`self.DynamicMaterialInstance`))
  (set `self.DT` DeltaSeconds)
  (`|ExecutionSequence`
    (:`then_0`
      ;[1 1 1] Animation Timer
      (if (`self.IsAnimating`)
        (bind _output_get (set `self.AnimationTimer` (+ (`self.DT`) (`self.AnimationTimer`))))
        (if (>= _output_get (`self.WaitTime`))
          (set `self.IsAnimating` false)
          (set `self.AnimationTimer` 0.0))))
    (:`then_1`
      ;[1 1 1] visibility based on mouse distance and facing value
      (bind _distance (`self.GetMouseDistanceFromSelf`))
      (`MaterialInstanceDynamic.SetScalarParameterValue` _dynamicmaterialinstance "MouseDistance" (- 1.0 (`KismetMathLibrary.FClamp` (/ _distance (`self.ClickableRadius`)))))
      (if (`self.VisibilityBasedOnFacingValue`)
        (`MaterialInstanceDynamic.SetScalarParameterValue` _dynamicmaterialinstance "Facing" (`KismetMathLibrary.Conv_BoolToDouble` (< (`self.GetFacingValue`) (- (* (/ (`self.ClickableAngle`) 360.0) 2.0) 1.0))))))
    (:`then_2`
      ;[1 1 1] Pressed Timer
      (if (`self.IsPressed`)
        (set `self.PressedTimer` (+ (`self.PressedTimer`) (`self.DT`)))
        (else
          (set `self.PressedTimer` 0.0))))))

(fn `CanBeAnimated`
  (returns (IsAnimatable :type Boolean))
  (locals (Animatable :type Boolean :default true))
  (if (`|EnumEquality` (`self.CarAnimation`) "NewEnumerator4")
    (set `local.Animatable` (not (`/Game/CarConfigurator/Car/Blueprints/BP_AudiA5.ConvertibleTopAnimating` (`self.Car`)))))
  (return (`local.Animatable`)))

(fn `Close`
  ;[1 1 1] Close event
  (set `self.IsOpen` false)
  (set `self.IsAnimating` true)
  (set `self.AnimationTimer` 0.0)
  (`GameplayStatics.PlaySoundAtLocation` (`self.CloseSound`) (`self.K2_GetActorLocation` self) (struct) 1.0 1.0 0.0 "/Game/CarConfigurator/Shared/Audio/Configurator_AmbientAttenuation.Configurator_AmbientAttenuation" null null)
  (`AudioComponent.Stop` (`self.AudioLoop`))
  (`/Game/CarConfigurator/Car/Blueprints/BP_AudiA5.StartAnimation` (`self.Car`) (`self.CloseSpeed`) (`self.CarAnimation`))
  ;[1 1 1] Move and hide focus point while animating
  (`self.K2_SetActorLocation` self (- (`self.K2_GetActorLocation` self) (`self.ClosePositionOffset`)) false false)
  (`MaterialInstanceDynamic.SetScalarParameterValue` (`self.DynamicMaterialInstance`) "WaitUntil" (+ (`GameplayStatics.GetTimeSeconds`) (`self.WaitTime`))))

(fn `ForceClose`
  (set `self.IsOpen` false)
  (`self.GetCarInstance`)
  (`self.Close`))

(fn `GetAnimationData`
  (bind _datatable (`self.DataTable`))
  (bind _outrownames (`DataTableFunctionLibrary.GetDataTableRowNames` _datatable))
  (for _array_element _outrownames
    (bind _returnvalue (`|GetDataTableRow` _datatable _array_element)
      (:`then`
        (bind (_carpart _opensound _closesound _loopingsound _openspeed _closespeed _waittime) (break `/Game/CarConfigurator/Shared/Blueprints/Car_Animation_Struct` _returnvalue))
        (if (`|EnumEquality` _carpart (`self.CarAnimation`))
          (set `self.OpenSound` _opensound)
          (set `self.CloseSound` _closesound)
          (set `self.LoopingSound` _loopingsound)
          (set `self.OpenSpeed` _openspeed)
          (set `self.CloseSpeed` _closespeed)
          (set `self.WaitTime` _waittime))))))

(fn `GetCarInstance`
  (bind _outactors (`GameplayStatics.GetAllActorsOfClass` "/Game/CarConfigurator/Car/Blueprints/BP_AudiA5.BP_AudiA5_C"))
  (set `self.Car` (`|GetArrayItem` _outactors)))

(fn `GetFacingValue`
  (returns (FacingValue :type "Float (double-precision)"))
  (bind _returnvalue (`KismetMathLibrary.Dot_VectorVector` (`self.GetActorRightVector` self) (`KismetMathLibrary.GetForwardVector` (`PlayerCameraManager.GetCameraRotation` (`PlayerController.PlayerCameraManager` (`GameplayStatics.GetPlayerController` 0))))))
  (if (`self.InvertFacingValue`)
    (return (* _returnvalue -1.0))
    (else
      (return _returnvalue))))

(fn `GetMouseDistanceFromSelf`
  (returns (Distance :type "Float (double-precision)"))
  (bind _returnvalue (`WidgetLayoutLibrary.GetMousePositionOnViewport`))
  (return (`KismetMathLibrary.Distance2D` _returnvalue (/ (`GameplayStatics.ProjectWorldToScreen` (`GameplayStatics.GetPlayerController` 0) (`self.K2_GetActorLocation` self)) (`WidgetLayoutLibrary.GetViewportScale`)))))

(fn `IsFocusPointClickable`
  (returns (isClickable :type Boolean))
  (bind _distance (`self.GetMouseDistanceFromSelf`))
  (if (`self.VisibilityBasedOnFacingValue`)
    (bind _returnvalue (< _distance (`self.ClickableRadius`)))
    (return (and _returnvalue (< (`self.GetFacingValue`) (- (* (/ (`self.ClickableAngle`) 360.0) 2.0) 1.0))))
    (else
      (return _returnvalue))))

(fn `Open`
  (bind _audioloop (`self.AudioLoop`))
  ;[1 1 1] Open event
  (set `self.IsOpen` true)
  (set `self.IsAnimating` true)
  (set `self.AnimationTimer` 0.0)
  (`GameplayStatics.PlaySoundAtLocation` (`self.OpenSound`) (`self.K2_GetActorLocation` self) (struct) 1.0 1.0 0.0 "/Game/CarConfigurator/Shared/Audio/Configurator_AmbientAttenuation.Configurator_AmbientAttenuation" null null)
  (`AudioComponent.SetSound` _audioloop (`self.LoopingSound`))
  (`AudioComponent.Play` _audioloop 1.0)
  (`/Game/CarConfigurator/Car/Blueprints/BP_AudiA5.StartAnimation` (`self.Car`) (`self.OpenSpeed`) (`self.CarAnimation`))
  ;[1 1 1] Move and hide focus point while animating
  (`self.K2_SetActorLocation` self (+ (`self.K2_GetActorLocation` self) (`self.ClosePositionOffset`)) false false)
  (`MaterialInstanceDynamic.SetScalarParameterValue` (`self.DynamicMaterialInstance`) "WaitUntil" (+ (`GameplayStatics.GetTimeSeconds`) (`self.WaitTime`))))

(fn `UserConstructionScript`)